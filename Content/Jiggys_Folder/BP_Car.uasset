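; BP_Car is the intro car, handling drive animations, opening dialogue and the handoff to the first-person character.
; DiologoStart updates each BC_Road, puts the paper away and shows a data-table subtitle.
; While the subtitle widget's InDiologo is set, keys 1–4 play a choice and its follow-up voice line.
; Addplayer moves the character to the exit point, blends the camera to theirs, then possesses them; old driving and dialogue-start chains are disconnected.
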(event `self.ReceiveBeginPlay`
  (bind _asbp_first_person_character (cast `/Game/FirstPerson/Blueprints/BP_FirstPersonCharacter` (`GameplayStatics.GetPlayerCharacter` 0)))
  (set `/Game/FirstPerson/Blueprints/BP_FirstPersonCharacter.Car` self _asbp_first_person_character)
  (set `self.Player` _asbp_first_person_character))

(event `Add player`
  (bind _camera (`self.Camera`))
  (bind _returnvalue (`SceneComponent.K2_GetComponentToWorld` (`self.PlayerOutPT`)))
  ; Player spawn
  (bind _returnvalue_2 (`GameplayStatics.GetActorOfClass` "/Game/FirstPerson/Blueprints/BP_FirstPersonCharacter.BP_FirstPersonCharacter_C"))
  (`SceneComponent.K2_SetWorldTransform` (`Actor.RootComponent` _returnvalue_2) (`KismetMathLibrary.MakeTransform` (.location _returnvalue) (`KismetMathLibrary.MakeRotator` 0.0 0.0 (- (.yaw (.rotation _returnvalue)) 90.0))) false false)
  (bind (_direction _newtrack_0) (`Timeline|Timeline`)
    (:`Update`
      (`SceneComponent.K2_SetWorldTransform` _camera (`KismetMathLibrary.TLerp` (`SceneComponent.K2_GetComponentToWorld` _camera) (`SceneComponent.K2_GetComponentToWorld` (`/Game/FirstPerson/Blueprints/BP_FirstPersonCharacter.FirstPersonCamera` _returnvalue_2)) _newtrack_0) false false))
    (:`Finished`
      (`Controller.Possess` (`GameplayStatics.GetPlayerController` 0) _returnvalue_2)
      (`self.SetActorHiddenInGame` _returnvalue_2 false)
      (`SceneComponent.SetVisibility` (`self.Arms`) true false)
      (`/Game/FirstPerson/Blueprints/BP_FirstPersonCharacter.Unload Menu` _returnvalue_2))))

(event `Player get out of car`
  ; Animations
  (`SkeletalMeshComponent.PlayAnimation` (`self.Arms`) "/Game/FirstPerson/PlayerArms/PlayerAnims/AS_Player_PlayerGetOut.AS_Player_PlayerGetOut" false))

(event `Car Start`
  ; Animations
  (`SkeletalMeshComponent.PlayAnimation` (`self.Car`) "/Game/Models/Car/CarAnims/AS_PlayerCar_DriveDown.AS_PlayerCar_DriveDown" false))

(event `Diologo Start`
  (bind (_datatable _rowname) (break `DataTableRowHandle` (`self.Entry Voice line`)))
  ; Stop road / put away paper
  (bind _outactors (`GameplayStatics.GetAllActorsOfClass` "/Game/Jiggys_Folder/BC_Road.BC_Road_C"))
  (for _array_element _outactors
    (set `/Game/Jiggys_Folder/BC_Road.Stop Road` false _array_element)
    (`SkeletalMeshComponent.PlayAnimation` (`self.Arms`) "/Game/FirstPerson/PlayerArms/PlayerAnims/AS_Player_DrivePaperPutAway.AS_Player_DrivePaperPutAway" false)
    (`KismetSystemLibrary.Delay` 0.2)
    (`SceneComponent.SetHiddenInGame` (`self.Paper`) true false)
    (bind _returnvalue (`|GetDataTableRow` _datatable _rowname)
      (:`then`
        (bind (_subtitles _voiceline _name _color) (break `/Game/Jiggys_Folder/Diaologo/S_Voicelines` _returnvalue))
        (`/Game/Jiggys_Folder/Diaologo/WB_Subtitles.Update Text` (`self.WB_Subtitttes`) (`KismetTextLibrary.Conv_TextToString` _subtitles) (`KismetTextLibrary.Conv_TextToString` _name) _color)))))

(event `Key|One`
  (params (Key :type "Key Structure"))
  ; Responding to Diologo
  (:`Pressed`
    (if (`/Game/Jiggys_Folder/Diaologo/WB_Subtitles.In diologo` (`self.WB_Subtitttes`))
      (set `/Game/Jiggys_Folder/Diaologo/WB_Subtitles.In diologo` false (`self.WB_Subtitttes`))
      (bind _returnvalue (`GameplayStatics.SpawnSound2D` "/Game/Audio/VoiceLines/Scene1/Scene1_DiaOption_1Understood.Scene1_DiaOption_1Understood" 1.0 1.0 0.0 null))
      (add `AudioComponent.OnAudioFinished` _returnvalue (delegate `Done1`)))))

(event `Done1`
  ; Responding to Diologo
  (`GameplayStatics.PlaySound2D` "/Game/Audio/VoiceLines/Scene1/Scene1_DiaIF_1Out.Scene1_DiaIF_1Out" 1.0 1.0 0.0 null null))

(event `Key|Two`
  (params (Key :type "Key Structure"))
  ; Responding to Diologo
  (:`Pressed`
    (if (`/Game/Jiggys_Folder/Diaologo/WB_Subtitles.In diologo` (`self.WB_Subtitttes`))
      (set `/Game/Jiggys_Folder/Diaologo/WB_Subtitles.In diologo` false (`self.WB_Subtitttes`))
      (bind _returnvalue (`GameplayStatics.SpawnSound2D` "/Game/Audio/VoiceLines/Scene1/Scene1_DiaOption_2Suprises.Scene1_DiaOption_2Suprises" 1.0 1.0 0.0 null))
      (add `AudioComponent.OnAudioFinished` _returnvalue (delegate `Done2`)))))

(event `Done2`
  ; Responding to Diologo
  (`GameplayStatics.PlaySound2D` "/Game/Audio/VoiceLines/Scene1/Scene1_DiaIF_2SAR.Scene1_DiaIF_2SAR" 1.0 1.0 0.0 null null))

(event `Key|Three`
  (params (Key :type "Key Structure"))
  ; Responding to Diologo
  (:`Pressed`
    (if (`/Game/Jiggys_Folder/Diaologo/WB_Subtitles.In diologo` (`self.WB_Subtitttes`))
      (set `/Game/Jiggys_Folder/Diaologo/WB_Subtitles.In diologo` false (`self.WB_Subtitttes`))
      (bind _returnvalue (`GameplayStatics.SpawnSound2D` "/Game/Audio/VoiceLines/Scene1/Scene1_DiaOption_3Byself.Scene1_DiaOption_3Byself" 1.0 1.0 0.0 null))
      (add `AudioComponent.OnAudioFinished` _returnvalue (delegate `Done3`)))))

(event `Done3`
  ; Responding to Diologo
  (`GameplayStatics.PlaySound2D` "/Game/Audio/VoiceLines/Scene1/Scene1_DiaIF_3Houston.Scene1_DiaIF_3Houston" 1.0 1.0 0.0 null null))

(event `Key|Four`
  (params (Key :type "Key Structure"))
  ; Responding to Diologo
  (:`Pressed`
    (if (`/Game/Jiggys_Folder/Diaologo/WB_Subtitles.In diologo` (`self.WB_Subtitttes`))
      (set `/Game/Jiggys_Folder/Diaologo/WB_Subtitles.In diologo` false (`self.WB_Subtitttes`))
      (bind _returnvalue (`GameplayStatics.SpawnSound2D` "/Game/Audio/VoiceLines/Scene1/Scene1_DiaOption_4Joker.Scene1_DiaOption_4Joker" 1.0 1.0 0.0 null))
      (add `AudioComponent.OnAudioFinished` _returnvalue (delegate `Done4`)))))

(event `Done4`
  ; Responding to Diologo
  (`GameplayStatics.PlaySound2D` "/Game/Audio/VoiceLines/Scene1/Scene1_DiaIF_4Job.Scene1_DiaIF_4Job" 1.0 1.0 0.0 null null))

(fn `UserConstructionScript`)