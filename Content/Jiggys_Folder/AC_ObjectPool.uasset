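; Actor component that keeps a pool of pre-spawned actors for reuse.
; InitializePool spawns instances of PooledActorClass in a PoolSize-driven loop and marks them unused; BeginPlay does not call it.
; SpawnFromPool linearly searches for the first actor not in use, moves it to the requested transform, marks it in use and returns it.
; The pool does not grow when every actor is busy.
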(event `self.ReceiveBeginPlay`)

(event `Initialize Pool`
  (for _ (range (+ (`self.Pool Size`) 1))
    (bind _pooled_actor_class (`self.Pooled Actor Class`)
      (:`then`
        (bind _returnvalue (`|SpawnActorFromClass` _pooled_actor_class (`KismetMathLibrary.MakeTransform` (0.0 0.0 0.0)) "Undefined" "MultiplyWithRoot" null null))
        (`KismetArrayLibrary.Array_AddUnique` (`self.Object Pool`) _returnvalue)
        (`/Game/Jiggys_Folder/BC_PoolActor.Set In use` _returnvalue false))
      (:`else`))))

(fn `Find First Availilble Actor`
  (returns (`Pooled Actor` :type "/Game/Jiggys_Folder/BC_PoolActor Object Reference"))
  (for _array_element (`self.Object Pool`)
    (if (not (`/Game/Jiggys_Folder/BC_PoolActor.In Use` _array_element))
      (return _array_element))))

(fn `Spawn From Pool`
  (params (`Spawn Transform` :type "Transform Structure"))
  (returns (`Pooled Actor` :type "/Game/Jiggys_Folder/BC_PoolActor Object Reference"))
  (bind _pooled_actor (`self.Find First Availilble Actor`))
  (`/Engine/EditorBlueprintResources/StandardMacros.IsValid` _pooled_actor
    (:`Is Valid`
      (`Actor.K2_SetActorTransform` _pooled_actor `Spawn Transform` false false)
      (`/Game/Jiggys_Folder/BC_PoolActor.Set In use` _pooled_actor true)
      (return _pooled_actor))))