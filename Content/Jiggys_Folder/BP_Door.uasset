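; BP_Door is a door that swings open and closed each time its RotateDoor event is called.
; A FlipFlop alternates between playing and reversing the DoorSwing timeline, whose track drives a yaw Lerp on the static mesh for a quarter-turn swing.
; The file also holds an unconnected FlipFlop that snaps the mesh between two yaws with debug prints and never runs.
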(event `Rotate Door`
  (`/Engine/EditorBlueprintResources/StandardMacros.FlipFlop`
    (:`A`
      (bind (_direction _newtrack_0) (`Timeline|Door Swing` :!label _label)
        (:`Update`
          (`SceneComponent.K2_SetRelativeRotation` (`self.StaticMesh`) (`KismetMathLibrary.MakeRotator` 0.0 0.0 (`KismetMathLibrary.Lerp` 0.0 90.0 _newtrack_0)) false false))))
    (:`B`
      (goto _label :!via `Reverse`))))

(fn `UserConstructionScript`)