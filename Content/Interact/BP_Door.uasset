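; BP_Door is an interactable skeletal-mesh door that is either a regular open/close door or a one-time shed door.
; BeginPlay picks animations from the ShedDoor flag, and RotateDoor plays them by DoorStatus unless locked.
; The shed door locks after opening and triggers Bp_TrapWire animations.
; A DoOnce with a delayed reset debounces input; opening also hides the player's interact icon if flagged.
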(event `self.ReceiveBeginPlay`
  ; What door is this?
  (if (`self.Shed Door`)
    (set `self.Ani Open` "/Game/Models/ShedAssets/ShedDoor/AS_ShedDoor_Opening.AS_ShedDoor_Opening")
    (set `self.Only open Once` true)
    (else
      (set `self.Ani Open` "/Game/Models/CabinAssets/Door/AS_DoorOpen_1.AS_DoorOpen_1")
      (set `self.Ani Close` "/Game/Models/CabinAssets/Door/AS_DoorClose_1.AS_DoorClose_1")
      (set `self.Only open Once` false))))

(event `Rotate Door`
  (if (not (`self.Is Locked`))
    (`/Engine/EditorBlueprintResources/StandardMacros.DoOnce` false :!label _label
      (:`Completed`
        (switch `/Game/Interact/E_Door` (`self.Door Status`)
          (:`NewEnumerator0`
            (`SkeletalMeshComponent.PlayAnimation` (`self.SkeletalMesh`) (`self.Ani Open`) false)
            (set `self.Door Status` "NewEnumerator1")
            (if (`self.Only open Once`)
              (set `self.Is Locked` true))
            (`|ExecutionSequence`
              (:`then_0`
                (`KismetSystemLibrary.Delay` 0.2)
                (if (`self.Icon`)
                  ; Icon only happens once
                  (bind _asbp_first_person_character (cast `/Game/FirstPerson/Blueprints/BP_FirstPersonCharacter` (`GameplayStatics.GetPlayerCharacter` 0)))
                  (`/Game/FirstPerson/Blueprints/BP_FirstPersonCharacter.Interact Icon` _asbp_first_person_character false)
                  (`self.Reset`)
                  (else
                    (`self.Reset`))))
              (:`then_1`
                ; If shed door play animation
                (if (`self.Shed Door`)
                  (bind _outactors (`GameplayStatics.GetAllActorsOfClass` "/Game/Models/ShedAssets/TrapWire/Bp_TrapWire.Bp_TrapWire_C"))
                  (`/Game/Models/ShedAssets/TrapWire/Bp_TrapWire.Play animation` _outactors)))))
          (:`NewEnumerator1`
            (if (not (`self.Only open Once`))
              (`SkeletalMeshComponent.PlayAnimation` (`self.SkeletalMesh`) (`self.Ani Close`) false)
              (set `self.Door Status` "NewEnumerator0")
              (`KismetSystemLibrary.Delay` 0.2)
              (`self.Reset`))))))))

(event `Reset`
  (goto _label :!via `Reset`))

(fn `UserConstructionScript`)